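; Base AI controller Blueprint that visualizes what its AI Perception component detects, for debugging.
; On each perception update it reads every updated actor's first last-sensed stimulus and checks whether it was successfully sensed and whether the actor is hostile.
; For each of the four spotted or lost, enemy or friend cases it draws a color-coded debug sphere at the stimulus location and prints a Polish status message.
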(event `self.ReceiveBeginPlay`)

(event `self.AIPerception.OnPerceptionUpdated`
  (params (UpdatedActors :type "Array of Actor Object Reference (by ref)"))
  (for _array_element UpdatedActors
    (bind _info (`AIPerceptionComponent.GetActorsPerception` (`self.AIPerception`) _array_element))
    (bind (_target _lastsensedstimuli _bishostile) (break `ActorPerceptionBlueprintInfo` _info))
    (bind (_output_age _output_expirationage _output_strength _output_stimuluslocation _output_receiverlocation _output_tag _output_bsuccessfullysensed) (break `AIStimulus` (`|GetArrayItem` _lastsensedstimuli)))
    (if _output_bsuccessfullysensed
      (if _bishostile
        (`KismetSystemLibrary.DrawDebugSphere` _output_stimuluslocation 50.0 12 (struct :`R` 1.0 :`A` 1.0) 3.0 2.0)
        (`KismetSystemLibrary.PrintString` "zauwazony wrog")
        (else
          (`KismetSystemLibrary.DrawDebugSphere` _output_stimuluslocation 50.0 12 (struct :`R` 0.024891 :`G` 1.0 :`A` 1.0) 3.0 2.0)
          (`KismetSystemLibrary.PrintString` "zauwazony przyjeciel")))
      (elif _bishostile
        (`KismetSystemLibrary.DrawDebugSphere` _output_stimuluslocation 50.0 12 (struct :`R` 1.0 :`G` 0.754848 :`A` 1.0) 3.0 2.0)
        (`KismetSystemLibrary.PrintString` "zgubiony wrog")
        (else
          (`KismetSystemLibrary.DrawDebugSphere` _output_stimuluslocation 50.0 12 (struct :`G` 0.236026 :`B` 1.0 :`A` 1.0) 3.0 2.0)
          (`KismetSystemLibrary.PrintString` "zgubiony przyjaciel"))))))

(fn `UserConstructionScript`)