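; Base character Blueprint for AI-controlled team members, assigning team identity and team color at spawn.
; On BeginPlay it looks up TeamName in DT_Teams, passes team, friend and enemy IDs to its AIControllerBase, then picks a red, blue, green or yellow mesh material by team ID.
; An optional TestMove flag walks the character forward on Tick until a time limit; without it, Tick disables itself.
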(event `self.ReceiveBeginPlay`
  (bind _mesh (`self.Mesh`))
  (bind _asaicontroller_base (cast `AIControllerBase` (`self.GetController`)))
  (bind _returnvalue (`|GetDataTableRow` "/Game/DT_Teams.DT_Teams" (`self.TeamName`))
    (:`then`
      (bind (_teamid _enemiesteamid _friendsteamid) (break `/Game/teams` _returnvalue))
      (`AIControllerBase.SetTeamProperties` _asaicontroller_base (make `TeamProperties` (`self.TeamName`) _teamid _friendsteamid _enemiesteamid))
      (bind (_returnvalue_teamname _returnvalue_aiteamid) (break `TeamProperties` (`AIControllerBase.GetTeamProperties` _asaicontroller_base)))
      (switch `int` _returnvalue_aiteamid
        (:`0`
          (`PrimitiveComponent.SetMaterial` _mesh 0 "/Game/Mannequin/Character/Materials/red.red"))
        (:`1`
          (`PrimitiveComponent.SetMaterial` _mesh 0 "/Game/Mannequin/Character/Materials/blue.blue"))
        (:`2`
          (`PrimitiveComponent.SetMaterial` _mesh 0 "/Game/Mannequin/Character/Materials/green.green"))
        (:`3`
          (`PrimitiveComponent.SetMaterial` _mesh 0 "/Game/Mannequin/Character/Materials/yellow.yellow"))))))

(event `self.ReceiveTick`
  (params (DeltaSeconds :type "Float (single-precision)"))
  (if (`self.testMove`)
    (if (<= (`GameplayStatics.GetRealTimeSeconds`) (`self.TimeForwardMove`))
      (`PawnMovementComponent.AddInputVector` (`self.CharacterMovement`) (`self.GetActorForwardVector`) false))
    (else
      (`self.SetActorTickEnabled` false))))

(fn `UserConstructionScript`)